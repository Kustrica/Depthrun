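; Player character Blueprint for Depthrun that adds debug hotkeys, a HUD click handler and a starting potion on top of existing character functionality.
; Y and U toggle god mode and super attack, while F3 toggles the adaptive debug widget through DepthrunHUD.
; Left mouse click asks the same HUD to close the chest reward, and BeginPlay grants one potion via PlayerEconomy.
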(event EventBeginPlay
  (Class|PlayerEconomy|AddPotions (Variables|Default|GetPlayerEconomy) 1))

(event Collision|EventActorBeginOverlap
  (params (OtherActor :type Actor%20Object%20Reference)))

(event EventTick
  (params (DeltaSeconds :type Float%20%28single-precision%29)))

(event Input|MouseEvents|LeftMouseButton
  (params (Key :type Key%20Structure :default "None"))
  (:Pressed
    (bind _asdepthrun_hud (Utilities|Casting|CastToDepthrunHUD (HUD|GetHUD (Game|GetPlayerController 0))))
    (Class|DepthrunHUD|CloseChestReward _asdepthrun_hud)))

(event Input|KeyboardEvents|F3
  (params (Key :type Key%20Structure :default "None"))
  (:Pressed
    (bind _asdepthrun_hud (Utilities|Casting|CastToDepthrunHUD (HUD|GetHUD (Game|GetPlayerController 0))))
    (Class|DepthrunHUD|ToggleAdaptiveDebugWidget _asdepthrun_hud)))

(event Input|KeyboardEvents|U
  (params (Key :type Key%20Structure :default "None"))
  (:Pressed
    (Class|DepthrunCharacter|ToggleSuperAttack)))

(event Input|KeyboardEvents|Y
  (params (Key :type Key%20Structure :default "None"))
  (:Pressed
    (Class|DepthrunCharacter|ToggleGodMode)))

(fn ConstructionScript)